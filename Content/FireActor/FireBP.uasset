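; FireBP is an actor that plays weapon fire audio, either as repeated shots or as a loop.
; Fire waits a random delay, resets counters and repeats an attached shot sound on a timer up to FireCount, while FireNew plays a loop for a fixed duration.
; Fire also starts a delayed hit timer, but its event is empty.
; The staged water, rock, hull and core impact sounds ahead of the actor are disconnected and never run.
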(event Custom|FireNew
  (Utilities|FlowControl|Delay (Math|Random|RandomFloatinRange 0.0 2.0))
  (CallFunction|Reset)
  (bind _returnvalue (Audio|SpawnSoundAttached (Variables|Default|GetFireLoopCue) (Variables|Default|GetDefaultSceneRoot) "None" "0, 0, 0" "0, 0, 0" "KeepRelativeOffset" false 1.0 1.0 0.0 0 0))
  (Variables|Default|SetAudioFireLoopComponent _returnvalue)
  (Utilities|FlowControl|Delay 5.0)
  (Audio|Components|Audio|Stop (Variables|Default|GetAudioFireLoopComponent)))

(event Custom|Timer_FireEvent
  (Audio|SpawnSoundAttached (Variables|Default|GetFireCue) (Variables|Default|GetDefaultSceneRoot) "None" "0, 0, 0" "0, 0, 0" "KeepRelativeOffset" false 1.0 1.0 0.0 0 0)
  (bind _output_get (Variables|Default|SetcurFireNumber (+ (Variables|Default|GetcurFireNumber) 1)))
  (if (>= _output_get (Variables|Default|GetFireCount))
    (Utilities|Time|ClearandInvalidateTimerbyHandle (Variables|Default|GetTimerHandle))))

(event Custom|Fire
  (Utilities|FlowControl|Delay (Math|Random|RandomFloatinRange 0.0 2.0))
  (CallFunction|Reset)
  (bind _returnvalue (Utilities|Time|SetTimerbyEvent (delegate Custom|Timer_FireEvent) (Variables|Default|GetIntervalTime) true))
  (Variables|Default|SetTimerHandle _returnvalue)
  (Utilities|FlowControl|Delay 1.5)
  (bind _returnvalue_2 (Utilities|Time|SetTimerbyEvent (delegate Custom|TimerHit) (Variables|Default|GetIntervalTime) true))
  (Variables|Default|SetHitHandle _returnvalue_2))

(event Custom|Reset
  (Variables|Default|SetcurFireNumber 0)
  (Variables|Default|SetcurHitWaterCount 0)
  (Variables|Default|SetcurHitRockCount 0)
  (Variables|Default|SetcurHitShipBodyCount 0)
  (Variables|Default|SetcurHitShipCoreCount 0))

(event Custom|TimerHit)

(fn ConstructionScript)